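; BP_Mushroom is a character that walks back and forth along the world X axis on its own.
; Tick feeds constant movement input in the direction set by IsFacingRight, which the side trigger boxes flip on overlap.
; The left box instead calls TouchedMessage on BPI_Touch implementers, while the right box always turns it left.
; Capsule and box overlaps also print debug strings.
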(event OnComponentBeginOverlap(CapsuleComponent)
  (params (OverlappedComponent :type Primitive%20Component%20Object%20Reference) (OtherActor :type Actor%20Object%20Reference) (OtherComp :type Primitive%20Component%20Object%20Reference) (OtherBodyIndex :type Integer) (bFromSweep :type Boolean) (SweepResult :type Hit%20Result%20Structure%20%28by%20ref%29))
  (Development|PrintString (Utilities|GetDisplayName OtherActor)))

(event OnComponentBeginOverlap(Box_Left)
  (params (OverlappedComponent :type Primitive%20Component%20Object%20Reference) (OtherActor :type Actor%20Object%20Reference) (OtherComp :type Primitive%20Component%20Object%20Reference) (OtherBodyIndex :type Integer) (bFromSweep :type Boolean) (SweepResult :type Hit%20Result%20Structure%20%28by%20ref%29))
  (if (Utilities|DoesObjectImplementInterface OtherActor "/Game/Blueprints/Interfaces/BPI_Touch.BPI_Touch_C")
    (Development|PrintString "Toqué al jugador.")
    (Class|BPITouch|Touched(Message) OtherActor)
    (else
      (Variables|Default|SetbIsFacingRight? true))))

(event OnComponentBeginOverlap(Box_Right)
  (params (OverlappedComponent :type Primitive%20Component%20Object%20Reference) (OtherActor :type Actor%20Object%20Reference) (OtherComp :type Primitive%20Component%20Object%20Reference) (OtherBodyIndex :type Integer) (bFromSweep :type Boolean) (SweepResult :type Hit%20Result%20Structure%20%28by%20ref%29))
  (Development|PrintString "Hello")
  (Variables|Default|SetbIsFacingRight? false))

(event EventBeginPlay
  (|CallParentFunction))

(event Collision|EventActorBeginOverlap
  (params (OtherActor :type Actor%20Object%20Reference))
  (|CallParentFunction OtherActor) ; This node is disabled and will not be called.\nDrag off pins to build functionality.
)

(event EventTick
  (params (DeltaSeconds :type Float%20%28single-precision%29))
  (|CallParentFunction DeltaSeconds)
  (if (Variables|Default|GetbIsFacingRight?)
    (Pawn|Input|AddMovementInput "1.000000,0.000000,0.000000" 1.0 false)
    (else
      (Pawn|Input|AddMovementInput "1.000000,0.000000,0.000000" -1.0 false))))

(fn ConstructionScript
  (|CallParentFunction))