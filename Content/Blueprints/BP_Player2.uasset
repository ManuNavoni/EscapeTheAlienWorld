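; Player character for a side-on 2D game, moving along the world X axis and jumping.
; On BeginPlay it registers the player Enhanced Input mapping context, whose move and jump actions drive the built-in movement and jump.
; The sprite is flipped by world rotation according to the sign of the movement input.
; A Touched event, or a capsule overlap with any BPI_Touch implementer, opens the Prototype level.
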(event OnComponentBeginOverlap(CapsuleComponent)
  (params (OverlappedComponent :type Primitive%20Component%20Object%20Reference) (OtherActor :type Actor%20Object%20Reference) (OtherComp :type Primitive%20Component%20Object%20Reference) (OtherBodyIndex :type Integer) (bFromSweep :type Boolean) (SweepResult :type Hit%20Result%20Structure%20%28by%20ref%29))
  (if (Utilities|DoesObjectImplementInterface OtherActor "/Game/Blueprints/Interfaces/BPI_Touch.BPI_Touch_C")
    (Game|OpenLevel(byName) "Prototype")))

(event Input|EnhancedActionEvents|EnhancedInputActionIA_Movement
  (params (ActionValue :type Float%20%28double-precision%29) (ElapsedSeconds :type Float%20%28double-precision%29) (TriggeredSeconds :type Float%20%28double-precision%29) (InputAction :type Input%20Action%20Object%20Reference :default "/Game/Input/IA_Movement.IA_Movement"))
  (Pawn|Input|AddMovementInput "1.000000,0.000000,0.000000" ActionValue false)
  (if (> ActionValue 0.0)
    (Transformation|SetWorldRotation (Variables|Default|GetSprite) "-0.000000,0.000000,-0.000000" false false)
    (else
      (Transformation|SetWorldRotation (Variables|Default|GetSprite) "-0.000000,-180.000000,-0.000000" false false))))

(event Input|EnhancedActionEvents|EnhancedInputActionIA_Jump
  (params (ActionValue :type Boolean) (ElapsedSeconds :type Float%20%28double-precision%29) (TriggeredSeconds :type Float%20%28double-precision%29) (InputAction :type Input%20Action%20Object%20Reference :default "/Game/Input/IA_Jump.IA_Jump"))
  (Character|Jump))

(event EventBeginPlay
  (Utilities|FlowControl|Sequence
    (:then_0
      (bind _asplayer_controller (Utilities|Casting|CastToPlayerController (Pawn|GetController)))
      (bind _output_get (Variables|Default|SetPlayer%20Controller _asplayer_controller))
      (Input|AddMappingContext (PlayerController|LocalPlayerSubsystems|GetEnhancedInputLocalPlayerSubsystem _output_get) "/Game/Input/IMC_Player.IMC_Player" 0 "(bIgnoreAllPressedKeysUntilRelease=True,bForceImmediately=False,bNotifyUserSettings=False)"))))

(event Collision|EventActorBeginOverlap
  (params (OtherActor :type Actor%20Object%20Reference)))

(event EventTick
  (params (DeltaSeconds :type Float%20%28single-precision%29)))

(event EventTouched
  (Game|OpenLevel(byName) "Prototype"))

(fn ConstructionScript)